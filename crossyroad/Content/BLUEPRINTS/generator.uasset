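; Endless lane generator for a Crossy Road-style chicken game, spawning grass, water, log, road and railroad rows along X.
; BeginPlay lays starting grass rows and several ten-row batches.
; Tick passes the chicken's X to CheckChickenLoc, which spawns another batch as it nears EndLoc.
; Spawnfloors rerolls at each nested branch, so row odds are uneven, and advances EndLoc; SpawnInitFloors is never called here.
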(event EventBeginPlay
  (for _index (range 0 3)
    (Game|SpawnActorfromClass "/Game/BLUEPRINTS/grass_spawn.grass_spawn_C" (Math|Transform|MakeTransform (Math|Vector|MakeVector (* (Math|Conversions|ToFloat(Integer) _index) -3e+01) 2e+01 1.0) "0, 0, 0" "1,1,1") "Undefined" 0 0)
    (for _index_2 (range 1 1)
      (CallFunction|Spawnfloors (Variables|Default|Getend_loc)))))

(event Collision|EventActorBeginOverlap
  (params (OtherActor :type Actor%20Object%20Reference)))

(event EventTick
  (params (DeltaSeconds :type Float%20%28single-precision%29))
  (bind _aschicken_bp (Utilities|Casting|CastTochicken_bp (Game|Player|GetPlayerPawn 0)))
  (CallFunction|CheckChickenLoc (.x (Transformation|GetActorLocation _aschicken_bp))))

(fn ConstructionScript)

(fn Spawnfloors
  (params (loc%20start :type Float%20%28single-precision%29))
  (bind _returnvalue (Math|Random|RandomInteger 5))
  (for _index (range 1 10)
    (if (== _returnvalue 0)
      (Game|SpawnActorfromClass "/Game/BLUEPRINTS/grass_spawn.grass_spawn_C" (Math|Transform|MakeTransform (Math|Vector|MakeVector (+ loc%20start (* _index 6e+01)) 2e+01 1.0) "0, 0, 0" "1,1,1") "Undefined" 0 0)
      (elif (== _returnvalue 1)
        (Game|SpawnActorfromClass "/Game/BLUEPRINTS/water_spawn.water_spawn_C" (Math|Transform|MakeTransform (Math|Vector|MakeVector (+ loc%20start (* _index 6e+01)) 2e+01 1.0) "0, 0, 0" "1,1,1") "Undefined" 0 0)
        (elif (== _returnvalue 2)
          (Game|SpawnActorfromClass "/Game/BLUEPRINTS/water_spawn_logs.water_spawn_logs_C" (Math|Transform|MakeTransform (Math|Vector|MakeVector (+ loc%20start (* _index 6e+01)) 2e+01 1.0) "0, 0, 0" "1,1,1") "Undefined" 0 0)
          (elif (== _returnvalue 3)
            (Game|SpawnActorfromClass "/Game/BLUEPRINTS/road_left_cars.road_left_cars_C" (Math|Transform|MakeTransform (Math|Vector|MakeVector (+ loc%20start (* _index 6e+01)) 2e+01 1.0) "0, 0, 0" "1,1,1") "Undefined" 0 0)
            (elif (== _returnvalue 4)
              (Game|SpawnActorfromClass "/Game/BLUEPRINTS/road_right_cars.road_right_cars_C" (Math|Transform|MakeTransform (Math|Vector|MakeVector (+ loc%20start (* _index 6e+01)) 2e+01 1.0) "0, 0, 0" "1,1,1") "Undefined" 0 0)
              (elif (== _returnvalue 5)
                (Game|SpawnActorfromClass "/Game/BLUEPRINTS/water_spawn_logs.water_spawn_logs_C" (Math|Transform|MakeTransform (Math|Vector|MakeVector (+ loc%20start (* _index 6e+01)) 2e+01 1.0) "0, 0, 0" "1,1,1") "Undefined" 0 0)
                (else
                  (Game|SpawnActorfromClass "/Game/BLUEPRINTS/railroad_spawn.railroad_spawn_C" (Math|Transform|MakeTransform (Math|Vector|MakeVector (+ loc%20start (* _index 6e+01)) 2e+01 1.0) "0, 0, 0" "1,1,1") "Undefined" 0 0)))))))))
  (Variables|Default|Setend_loc (+ loc%20start 6e+02)))

(fn SpawnInitFloors
  (for _index (range 0 2)
    (Utilities|IsValid 0
      (:Is%20Valid
        (CallFunction|Spawnfloors 0.0))
      (:Is%20Not%20Valid
        (CallFunction|Spawnfloors (.x (Transformation|GetActorLocation (Game|Player|GetPlayerPawn 0))))))))

(fn CheckChickenLoc
  (params (x%20loc :type Float%20%28single-precision%29))
  (if (>= x%20loc (- (Variables|Default|Getend_loc) 2e+02))
    (CallFunction|Spawnfloors (Variables|Default|Getend_loc))))