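; Road row actor that builds a strip of road and spawns left-side car traffic on it.
; On BeginPlay it spawns four Road pieces along Y by a spacer; only the first two are offset from the actor's own Y.
; Each Tick makes a 1-in-200 random roll to spawn one of two left car classes at a set Y, using the actor's X and Z.
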(event EventBeginPlay
  (CallFunction|Spawnroad (Transformation|GetActorLocation)))

(event Collision|EventActorBeginOverlap
  (params (OtherActor :type Actor%20Object%20Reference)))

(event EventTick
  (params (DeltaSeconds :type Float%20%28single-precision%29))
  (CallFunction|Spawncars (Transformation|GetActorLocation)))

(fn ConstructionScript)

(fn Spawnroad
  (params (Spawn%20Transform%20Location :type Vector))
  (bind _spacer (Variables|Default|Getspacer))
  (Game|SpawnActorfromClass "/Game/BLUEPRINTS/road.road_C" (Math|Transform|MakeTransform (Math|Vector|MakeVector (.x Spawn%20Transform%20Location) (.y Spawn%20Transform%20Location) (.z Spawn%20Transform%20Location)) "0, 0, 0" "1,1,1") "Undefined" 0 0)
  (Game|SpawnActorfromClass "/Game/BLUEPRINTS/road.road_C" (Math|Transform|MakeTransform (Math|Vector|MakeVector (.x Spawn%20Transform%20Location) (+ (.y Spawn%20Transform%20Location) _spacer) (.z Spawn%20Transform%20Location)) "0, 0, 0" "1,1,1") "Undefined" 0 0)
  (Game|SpawnActorfromClass "/Game/BLUEPRINTS/road.road_C" (Math|Transform|MakeTransform (Math|Vector|MakeVector (.x Spawn%20Transform%20Location) (* 2.0 _spacer) (.z Spawn%20Transform%20Location)) "0, 0, 0" "1,1,1") "Undefined" 0 0)
  (Game|SpawnActorfromClass "/Game/BLUEPRINTS/road.road_C" (Math|Transform|MakeTransform (Math|Vector|MakeVector (.x Spawn%20Transform%20Location) (* 3.0 _spacer) (.z Spawn%20Transform%20Location)) "0, 0, 0" "1,1,1") "Undefined" 0 0))

(fn Spawncars
  (params (spawn%20location :type Vector))
  (bind _yspawn (Variables|Default|Getyspawn))
  (if (== (Math|Conversions|ToFloat(Integer) (Math|Random|RandomInteger 200)) 1.0)
    (if (Math|Boolean|Equal(Boolean) (Math|Random|RandomBool) true)
      (Game|SpawnActorfromClass "/Game/BLUEPRINTS/car1-left.car1-left_C" (Math|Transform|MakeTransform (Math|Vector|MakeVector (.x spawn%20location) _yspawn (.z spawn%20location)) "0, 0, 0" "1,1,1") "Undefined" 0 0)
      (else
        (Game|SpawnActorfromClass "/Game/BLUEPRINTS/car2-left1.car2-left1_C" (Math|Transform|MakeTransform (Math|Vector|MakeVector (.x spawn%20location) _yspawn (.z spawn%20location)) "0, 0, 0" "1,1,1") "Undefined" 0 0)))))