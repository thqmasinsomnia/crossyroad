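; Spawner actor that lays down water and randomly releases logs at its location.
; On BeginPlay it spawns three Water actors along Y using Spacer, though the third takes Spacer times two as absolute Y, ignoring the spawner's Y.
; Every Tick it has a one-in-100 chance to spawn a Log at its own location, so log frequency depends on frame rate.
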(event EventBeginPlay
  (CallFunction|Spawnwater (Transformation|GetActorLocation)))

(event Collision|EventActorBeginOverlap
  (params (OtherActor :type Actor%20Object%20Reference)))

(event EventTick
  (params (DeltaSeconds :type Float%20%28single-precision%29))
  (CallFunction|SpawnLogs (Transformation|GetActorLocation)))

(fn ConstructionScript)

(fn Spawnwater
  (params (Spawn%20Transform%20Location :type Vector))
  (bind _spacer (Variables|Default|Getspacer))
  (Game|SpawnActorfromClass "/Game/BLUEPRINTS/water.water_C" (Math|Transform|MakeTransform (Math|Vector|MakeVector (.x Spawn%20Transform%20Location) (.y Spawn%20Transform%20Location) (.z Spawn%20Transform%20Location)) "0, 0, 0" "1,1,1") "Undefined" 0 0)
  (Game|SpawnActorfromClass "/Game/BLUEPRINTS/water.water_C" (Math|Transform|MakeTransform (Math|Vector|MakeVector (.x Spawn%20Transform%20Location) (+ (.y Spawn%20Transform%20Location) _spacer) (.z Spawn%20Transform%20Location)) "0, 0, 0" "1,1,1") "Undefined" 0 0)
  (Game|SpawnActorfromClass "/Game/BLUEPRINTS/water.water_C" (Math|Transform|MakeTransform (Math|Vector|MakeVector (.x Spawn%20Transform%20Location) (* _spacer 2.0) (.z Spawn%20Transform%20Location)) "0, 0, 0" "1,1,1") "Undefined" 0 0))

(fn SpawnLogs
  (params (spawn%20location :type Vector))
  (if (== (Math|Conversions|ToFloat(Integer) (Math|Random|RandomInteger 100)) 1.0)
    (Game|SpawnActorfromClass "/Game/BLUEPRINTS/log.log_C" (Math|Transform|MakeTransform (Math|Vector|MakeVector (.x spawn%20location) (.y spawn%20location) (.z spawn%20location)) "0, 0, 0" "1,1,1") "Undefined" 0 0)))