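; Player-controllable chicken pawn that moves from forward and right axis input.
; The axis events add movement input along the actor's forward and right vectors, scaled by MaxSpeed.
; Tick consumes that vector, scales it by delta time and applies it as an unswept local offset, so the world-space directions get treated as local and movement skips collision.
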(event EventBeginPlay)

(event Collision|EventActorBeginOverlap
  (params (OtherActor :type Actor%20Object%20Reference)))

(event EventTick
  (params (DeltaSeconds :type Float%20%28single-precision%29))
  (bind _returnvalue (Class|Pawn|ConsumeMovementInputVector))
  (Transformation|AddActorLocalOffset (* _returnvalue DeltaSeconds) false false))

(event Input|AxisEvents|InputAxismove_forward
  (params (AxisValue :type Float%20%28single-precision%29))
  ;[1 1 1] movements
  (Pawn|Input|AddMovementInput (Transformation|GetActorForwardVector) (* AxisValue (Variables|Default|Getmax_speed)) false))

(event Input|AxisEvents|InputAxismove_right
  (params (AxisValue :type Float%20%28single-precision%29))
  ;[1 1 1] movements
  (Pawn|Input|AddMovementInput (Transformation|GetActorRightVector) (* AxisValue (Variables|Default|Getmax_speed)) false))

(fn ConstructionScript)