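; Spawner actor that lays out a strip of water with scattered lilypads, apparently as a lane for the chicken player.
; On BeginPlay it spawns four Water actors along Y (the last two at absolute Spacer multiples), then a random number of Lillypads at random absolute Y.
; KillSelf runs only once, right after spawning, destroying the spawner if chicken_bp is over 500 units ahead in X.
; SpawnRocks is defined but never called.
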(event EventBeginPlay
  (bind _returnvalue (Transformation|GetActorLocation))
  (CallFunction|Spawnwater _returnvalue)
  (CallFunction|SpawnLilys _returnvalue)
  (CallFunction|KillSelf))

(event Collision|EventActorBeginOverlap
  (params (OtherActor :type Actor%20Object%20Reference)))

(event EventTick
  (params (DeltaSeconds :type Float%20%28single-precision%29)))

(fn ConstructionScript)

(fn Spawnwater
  (params (Spawn%20Transform%20Location :type Vector))
  (bind _spacer (Variables|Default|Getspacer))
  (Game|SpawnActorfromClass "/Game/BLUEPRINTS/water.water_C" (Math|Transform|MakeTransform (Math|Vector|MakeVector (.x Spawn%20Transform%20Location) (.y Spawn%20Transform%20Location) (.z Spawn%20Transform%20Location)) "0, 0, 0" "1,1,1") "Undefined" 0 0)
  (Game|SpawnActorfromClass "/Game/BLUEPRINTS/water.water_C" (Math|Transform|MakeTransform (Math|Vector|MakeVector (.x Spawn%20Transform%20Location) (+ (.y Spawn%20Transform%20Location) _spacer) (.z Spawn%20Transform%20Location)) "0, 0, 0" "1,1,1") "Undefined" 0 0)
  (Game|SpawnActorfromClass "/Game/BLUEPRINTS/water.water_C" (Math|Transform|MakeTransform (Math|Vector|MakeVector (.x Spawn%20Transform%20Location) (* _spacer 2.0) (.z Spawn%20Transform%20Location)) "0, 0, 0" "1,1,1") "Undefined" 0 0)
  (Game|SpawnActorfromClass "/Game/BLUEPRINTS/water.water_C" (Math|Transform|MakeTransform (Math|Vector|MakeVector (.x Spawn%20Transform%20Location) (* _spacer 3.0) (.z Spawn%20Transform%20Location)) "0, 0, 0" "1,1,1") "Undefined" 0 0))

(fn SpawnLilys
  (params (spawn%20location :type Vector))
  (for _index (range 0 (Math|Random|RandomInteger 10))
    (Game|SpawnActorfromClass "/Game/BLUEPRINTS/lillypad.lillypad_C" (Math|Transform|MakeTransform (Math|Vector|MakeVector (.x spawn%20location) (Math|Conversions|ToFloat(Integer) (Math|Random|RandomInteger 500)) (.z spawn%20location)) "0, 0, 0" "1,1,1") "Undefined" 0 0)))

(fn SpawnRocks
  (params (spawn%20location :type Vector))
  (for _index (range 0 (Math|Random|RandomInteger 5))
    (Game|SpawnActorfromClass "/Game/BLUEPRINTS/rock.rock_C" (Math|Transform|MakeTransform (Math|Vector|MakeVector (.x spawn%20location) (Math|Conversions|ToFloat(Integer) (Math|Random|RandomInteger 500)) (.z spawn%20location)) "0, 0, 0" "1,1,1") "Undefined" 0 0)))

(fn KillSelf
  (bind _aschicken_bp (Utilities|Casting|CastTochicken_bp (Game|Player|GetPlayerPawn 0)))
  (if (> (.x (Transformation|GetActorLocation _aschicken_bp)) (+ (.x (Transformation|GetActorLocation)) 5e+02))
    (Actor|DestroyActor)))