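; Grass lane spawner actor that populates one strip of terrain for the chicken player to travel across.
; On BeginPlay it spawns a row of four grass tiles spaced along Y, then random numbers of trees and rocks and an occasional coin at random Y positions on the same X.
; Every Tick it destroys itself once the chicken pawn is more than a set distance ahead in X, leaving the spawned actors to themselves.
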(event EventBeginPlay
  (bind _returnvalue (Transformation|GetActorLocation))
  (CallFunction|Spawngrass _returnvalue)
  (CallFunction|SpawnTrees _returnvalue)
  (CallFunction|SpawnRocks _returnvalue)
  (CallFunction|SpawnCoin _returnvalue))

(event Collision|EventActorBeginOverlap
  (params (OtherActor :type Actor%20Object%20Reference)))

(event EventTick
  (params (DeltaSeconds :type Float%20%28single-precision%29))
  (CallFunction|KillSelf))

(fn ConstructionScript)

(fn Spawngrass
  (params (Spawn%20Transform%20Location :type Vector))
  (bind _spacer (Variables|Default|Getspacer))
  (Game|SpawnActorfromClass "/Game/BLUEPRINTS/grass.grass_C" (Math|Transform|MakeTransform (Math|Vector|MakeVector (.x Spawn%20Transform%20Location) (.y Spawn%20Transform%20Location) (.z Spawn%20Transform%20Location)) "0, 0, 0" "1,1,1") "Undefined" 0 0)
  (Game|SpawnActorfromClass "/Game/BLUEPRINTS/grass.grass_C" (Math|Transform|MakeTransform (Math|Vector|MakeVector (.x Spawn%20Transform%20Location) (+ (.y Spawn%20Transform%20Location) _spacer) (.z Spawn%20Transform%20Location)) "0, 0, 0" "1,1,1") "Undefined" 0 0)
  (Game|SpawnActorfromClass "/Game/BLUEPRINTS/grass.grass_C" (Math|Transform|MakeTransform (Math|Vector|MakeVector (.x Spawn%20Transform%20Location) (* _spacer 2.0) (.z Spawn%20Transform%20Location)) "0, 0, 0" "1,1,1") "Undefined" 0 0)
  (Game|SpawnActorfromClass "/Game/BLUEPRINTS/grass.grass_C" (Math|Transform|MakeTransform (Math|Vector|MakeVector (.x Spawn%20Transform%20Location) (* _spacer 3.0) (.z Spawn%20Transform%20Location)) "0, 0, 0" "1,1,1") "Undefined" 0 0))

(fn SpawnTrees
  (params (spawn%20location :type Vector))
  (for _index (range 1 (Math|Random|RandomInteger 7))
    (Game|SpawnActorfromClass "/Game/BLUEPRINTS/tree.tree_C" (Math|Transform|MakeTransform (Math|Vector|MakeVector (.x spawn%20location) (Math|Conversions|ToFloat(Integer) (Math|Random|RandomInteger 1000)) (.z spawn%20location)) "0, 0, 0" "1,1,1") "Undefined" 0 0)))

(fn SpawnRocks
  (params (spawn%20location :type Vector))
  (for _index (range 0 (Math|Random|RandomInteger 5))
    (Game|SpawnActorfromClass "/Game/BLUEPRINTS/rock.rock_C" (Math|Transform|MakeTransform (Math|Vector|MakeVector (.x spawn%20location) (Math|Conversions|ToFloat(Integer) (Math|Random|RandomInteger 500)) (.z spawn%20location)) "0, 0, 0" "1,1,1") "Undefined" 0 0)))

(fn KillSelf
  (bind _aschicken_bp (Utilities|Casting|CastTochicken_bp (Game|Player|GetPlayerPawn 0)))
  (if (> (.x (Transformation|GetActorLocation _aschicken_bp)) (+ (.x (Transformation|GetActorLocation)) 5e+02))
    (Actor|DestroyActor)))

(fn SpawnCoin
  (params (spawn%20location :type Vector))
  (if (== (Math|Random|RandomInteger 3) 1)
    (Game|SpawnActorfromClass "/Game/BLUEPRINTS/coin.coin_C" (Math|Transform|MakeTransform (Math|Vector|MakeVector (.x spawn%20location) (Math|Conversions|ToFloat(Integer) (Math|Random|RandomInteger 500)) (.z spawn%20location)) "0, 0, 0" "1,1,1") "Undefined" 0 0)))