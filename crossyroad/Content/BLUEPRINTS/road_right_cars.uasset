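; A road lane spawner that lays road pieces and feeds rightward traffic into the level, apparently for a chicken road-crossing game.
; On BeginPlay it spawns four Road actors spaced along Y.
; Each tick it has a small random chance to spawn one of four car or truck types at a Y offset.
; It also destroys itself once the chicken player pawn is far enough past it on X.
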(event EventBeginPlay
  (CallFunction|Spawnroad (Transformation|GetActorLocation)))

(event Collision|EventActorBeginOverlap
  (params (OtherActor :type Actor%20Object%20Reference)))

(event EventTick
  (params (DeltaSeconds :type Float%20%28single-precision%29))
  (CallFunction|Spawncars (Transformation|GetActorLocation))
  (CallFunction|KillSelf))

(fn ConstructionScript)

(fn Spawnroad
  (params (Spawn%20Transform%20Location :type Vector))
  (bind _spacer (Variables|Default|Getspacer))
  (Game|SpawnActorfromClass "/Game/BLUEPRINTS/road.road_C" (Math|Transform|MakeTransform (Math|Vector|MakeVector (.x Spawn%20Transform%20Location) (.y Spawn%20Transform%20Location) (.z Spawn%20Transform%20Location)) "0, 0, 0" "1,1,1") "Undefined" 0 0)
  (Game|SpawnActorfromClass "/Game/BLUEPRINTS/road.road_C" (Math|Transform|MakeTransform (Math|Vector|MakeVector (.x Spawn%20Transform%20Location) (+ (.y Spawn%20Transform%20Location) _spacer) (.z Spawn%20Transform%20Location)) "0, 0, 0" "1,1,1") "Undefined" 0 0)
  (Game|SpawnActorfromClass "/Game/BLUEPRINTS/road.road_C" (Math|Transform|MakeTransform (Math|Vector|MakeVector (.x Spawn%20Transform%20Location) (* _spacer 2.0) (.z Spawn%20Transform%20Location)) "0, 0, 0" "1,1,1") "Undefined" 0 0)
  (Game|SpawnActorfromClass "/Game/BLUEPRINTS/road.road_C" (Math|Transform|MakeTransform (Math|Vector|MakeVector (.x Spawn%20Transform%20Location) (* _spacer 3.0) (.z Spawn%20Transform%20Location)) "0, 0, 0" "1,1,1") "Undefined" 0 0))

(fn Spawncars
  (params (spawn%20location :type Vector))
  (bind _returnvalue (+ (.y spawn%20location) 1e+03))
  (if (== (Math|Conversions|ToFloat(Integer) (Math|Random|RandomInteger 100)) 1.0)
    (switch int (Math|Random|RandomInteger 4)
      (:0
        (Game|SpawnActorfromClass "/Game/BLUEPRINTS/car2-right.car2-right_C" (Math|Transform|MakeTransform (Math|Vector|MakeVector (.x spawn%20location) _returnvalue (.z spawn%20location)) "0, 0, 0" "1,1,1") "Undefined" 0 0))
      (:1
        (Game|SpawnActorfromClass "/Game/BLUEPRINTS/car1-right.car1-right_C" (Math|Transform|MakeTransform (Math|Vector|MakeVector (.x spawn%20location) _returnvalue (.z spawn%20location)) "0, 0, 0" "1,1,1") "Undefined" 0 0))
      (:2
        (Game|SpawnActorfromClass "/Game/BLUEPRINTS/truck1-right.truck1-right_C" (Math|Transform|MakeTransform (Math|Vector|MakeVector (.x spawn%20location) _returnvalue (.z spawn%20location)) "0, 0, 0" "1,1,1") "Undefined" 0 0))
      (:3
        (Game|SpawnActorfromClass "/Game/BLUEPRINTS/truck2-right.truck2-right_C" (Math|Transform|MakeTransform (Math|Vector|MakeVector (.x spawn%20location) _returnvalue (.z spawn%20location)) "0, 0, 0" "1,1,1") "Undefined" 0 0)))))

(fn KillSelf
  (bind _aschicken_bp (Utilities|Casting|CastTochicken_bp (Game|Player|GetPlayerPawn 0)))
  (if (> (.x (Transformation|GetActorLocation _aschicken_bp)) (+ (.x (Transformation|GetActorLocation)) 5e+02))
    (Actor|DestroyActor)))