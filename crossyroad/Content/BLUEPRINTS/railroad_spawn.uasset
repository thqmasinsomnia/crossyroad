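; Railroad spawner actor that lays track and sends trains across it, removing itself once the chicken player passes it.
; On BeginPlay it spawns four Railroad pieces spaced along Y, the last two at absolute rather than relative offsets.
; Each Tick has a small random chance to spawn a row of Train actors along Y.
; KillSelf runs each Tick, destroying the spawner when the player is far enough ahead in X.
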(event EventBeginPlay
  (CallFunction|SpawnRailroad (Transformation|GetActorLocation)))

(event Collision|EventActorBeginOverlap
  (params (OtherActor :type Actor%20Object%20Reference)))

(event EventTick
  (params (DeltaSeconds :type Float%20%28single-precision%29))
  (CallFunction|KillSelf)
  (if (== (Math|Random|RandomInteger 200) 10)
    (CallFunction|SpawnTrain (Transformation|GetActorLocation))
    (CallFunction|KillSelf)))

(fn ConstructionScript)

(fn SpawnRailroad
  (params (Spawn%20Transform%20Location :type Vector))
  (bind _spacer (Variables|Default|Getspacer))
  (Game|SpawnActorfromClass "/Game/BLUEPRINTS/railroad.railroad_C" (Math|Transform|MakeTransform (Math|Vector|MakeVector (.x Spawn%20Transform%20Location) (.y Spawn%20Transform%20Location) (.z Spawn%20Transform%20Location)) "0, 0, 0" "1,1,1") "Undefined" 0 0)
  (Game|SpawnActorfromClass "/Game/BLUEPRINTS/railroad.railroad_C" (Math|Transform|MakeTransform (Math|Vector|MakeVector (.x Spawn%20Transform%20Location) (+ (.y Spawn%20Transform%20Location) _spacer) (.z Spawn%20Transform%20Location)) "0, 0, 0" "1,1,1") "Undefined" 0 0)
  (Game|SpawnActorfromClass "/Game/BLUEPRINTS/railroad.railroad_C" (Math|Transform|MakeTransform (Math|Vector|MakeVector (.x Spawn%20Transform%20Location) (* 2.0 _spacer) (.z Spawn%20Transform%20Location)) "0, 0, 0" "1,1,1") "Undefined" 0 0)
  (Game|SpawnActorfromClass "/Game/BLUEPRINTS/railroad.railroad_C" (Math|Transform|MakeTransform (Math|Vector|MakeVector (.x Spawn%20Transform%20Location) (* 3.0 _spacer) (.z Spawn%20Transform%20Location)) "0, 0, 0" "1,1,1") "Undefined" 0 0))

(fn SpawnTrain
  (params (spawn%20location :type Vector))
  (for _index (range 0 10)
    (bind _output_get (Variables|Default|Setyspawn (+ (Variables|Default|Getyspawn) 5e+01)))
    (Game|SpawnActorfromClass "/Game/BLUEPRINTS/train.train_C" (Math|Transform|MakeTransform (Math|Vector|MakeVector (.x spawn%20location) _output_get (.z spawn%20location)) "0, 0, 0" "1,1,1") "Undefined" 0 0))
  (Variables|Default|Setyspawn 2e+03))

(fn KillSelf
  (bind _aschicken_bp (Utilities|Casting|CastTochicken_bp (Game|Player|GetPlayerPawn 0)))
  (if (> (.x (Transformation|GetActorLocation _aschicken_bp)) (+ (.x (Transformation|GetActorLocation)) 5e+02))
    (Actor|DestroyActor)))