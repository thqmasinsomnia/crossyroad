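; Train obstacle actor that speeds along its local negative Y axis in a game with a chicken player pawn.
; Each Tick lowers a stored offset and applies it as a local move, so the train accelerates frame by frame without delta-time scaling.
; It destroys itself once its world Y drops below a lower bound or the chicken gets far enough ahead of it along world X.
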(event EventBeginPlay)

(event Collision|EventActorBeginOverlap
  (params (OtherActor :type Actor%20Object%20Reference)))

(event EventTick
  (params (DeltaSeconds :type Float%20%28single-precision%29))
  (CallFunction|KillSelf)
  (CallFunction|KillifOutofbounds)
  (bind _output_get (Variables|Default|SetNewVar_0 (+ (Variables|Default|GetNewVar_0) -0.1)))
  (Class|Actor|AddActorLocalTransform (Math|Transform|MakeTransform (Math|Vector|MakeVector 0.0 _output_get 0.0) "0, 0, 0" "1,1,1") false false))

(fn ConstructionScript)

(fn KillifOutofbounds
  (if (< (.y (Transformation|GetActorLocation)) -2e+02)
    (Actor|DestroyActor)))

(fn KillSelf
  (bind _aschicken_bp (Utilities|Casting|CastTochicken_bp (Game|Player|GetPlayerPawn 0)))
  (if (> (.x (Transformation|GetActorLocation _aschicken_bp)) (+ (.x (Transformation|GetActorLocation)) 5e+02))
    (Actor|DestroyActor)))