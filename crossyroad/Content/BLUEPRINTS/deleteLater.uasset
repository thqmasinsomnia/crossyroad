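; Scratch Character Blueprint named deleteLater that experiments with basic movement.
; Tick consumes the pending movement input vector and applies it, scaled by delta time, as an unswept local offset.
; A separate MoveForward function calls Jump, then sweeps the actor a fixed distance along its forward vector while setting a fixed absolute rotation.
; BeginPlay, overlap and construction logic are empty, and nothing in the graphs calls MoveForward.
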(event EventBeginPlay)

(event Collision|EventActorBeginOverlap
  (params (OtherActor :type Actor%20Object%20Reference)))

(event EventTick
  (params (DeltaSeconds :type Float%20%28single-precision%29))
  (bind _returnvalue (Class|Pawn|ConsumeMovementInputVector))
  (Transformation|AddActorLocalOffset (* _returnvalue DeltaSeconds) false false))

(fn ConstructionScript)

(fn MoveForward
  (Character|Jump)
  (Transformation|SetActorLocationAndRotation (+ (Transformation|GetActorLocation) (* (Transformation|GetActorForwardVector) 2e+02)) (Math|Rotator|MakeRotator 0.0 0.0 -1.0) true))